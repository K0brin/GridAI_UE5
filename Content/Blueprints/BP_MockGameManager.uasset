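; BP_MockGameManager is a manager actor that opens the main menu and can tear the current game down back to it.
; On BeginPlay it shows the cursor, creates UI_MainMenuWidget, passes itself as MockManager and enables input.
; Pressing 1 re-adds the menu and destroys all BP_GridComponent, BP_MainCharacter and BP_Enemy actors.
; The destroy loops are nested, so characters are cleared only if a grid exists, and enemies only if a character also exists.
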(event EventBeginPlay
  (Variables|/Script/Engine.PlayerController|SetbShowMouseCursor (Game|GetPlayerController 0) true)
  (bind _returnvalue (UserInterface|CreateWidget "/Game/UI/UI_MainMenuWidget.UI_MainMenuWidget_C"))
  (bind _output_get (Variables|Default|SetUIElement _returnvalue))
  (UserInterface|Viewport|AddtoViewport _output_get 0)
  (Variables|/Game/UI/UI_MainMenuWidget.UI_MainMenuWidget_C|SetMockManager (Variables|Default|GetUIElement) self)
  (Input|EnableInput (Game|GetPlayerController 0)))

(event Collision|EventActorBeginOverlap
  (params (OtherActor :type Actor%20Object%20Reference)))

(event EventTick
  (params (DeltaSeconds :type Float%20%28single-precision%29)))

(event Input|KeyboardEvents|1
  (params (Key :type Key%20Structure :default "None"))
  (:Pressed
    (UserInterface|Viewport|AddtoViewport (Variables|Default|GetUIElement) 0)
    (bind _outactors (Actor|GetAllActorsOfClass "/Game/Blueprints/BP_GridComponent.BP_GridComponent_C"))
    (for _array_element _outactors
      (Actor|DestroyActor _array_element)
      (bind _outactors_2 (Actor|GetAllActorsOfClass "/Game/Blueprints/BP_MainCharacter.BP_MainCharacter_C"))
      (for _array_element_2 _outactors_2
        (Actor|DestroyActor _array_element_2)
        (bind _outactors_3 (Actor|GetAllActorsOfClass "/Game/Blueprints/BP_Enemy.BP_Enemy_C"))
        (for _array_element_3 _outactors_3
          (Actor|DestroyActor _array_element_3))))))

(fn ConstructionScript)